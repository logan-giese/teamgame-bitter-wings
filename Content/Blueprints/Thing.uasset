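; Player-controlled plane for a race, flown with pitch, yaw, roll and throttle input, with roll input ignored near the ground.
; A looping timer raises integer speed while Forward is held and lowers it otherwise.
; Tick sets angular velocity from the axes, scaled by height-based air control, and blends linear velocity toward forward times speed.
; Throttle press and release set smoke opacity through a Material Parameter Collection; power-up only prints.
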(event EventBeginPlay
  (Variables|Default|SetOpacityVar "/Game/Materials/m_SMoke.m_Smoke")
  (Utilities|Time|SetTimerbyFunctionName 0 "ThrottleInput" 0.05 true))

(event EventTick
  (params (DeltaSeconds :type Float%20%28single-precision%29))
  ;[0.7317 1 0.2878] Changes the air control variable for takeoff and for flying to make it slower in air
  (if (< (.z (Transformation|GetWorldLocation (Variables|Default|GetPlane))) 3e+01)
    (Variables|Default|SetAirControl 1.65e+03)
    (else
      (Variables|Default|SetAirControl 7e+01)))
  (CallFunction|ApplyTurning)
  (CallFunction|CalculateSpeed))

(event Input|ActionEvents|InputActionForward
  (params (Key :type Key%20Structure :default "None"))
  (:Pressed
    (bind _output_get (Variables|Default|SetForward true))
    ;[1 1 1] Smoke trails defined by throttle bool only
    (Rendering|Material|SetScalarParameterValue "/Game/Materials/mc_Opacity.mc_Opacity" "Opacity Scalar" (Math|Float|Clamp(Float) (* (Math|Conversions|ToInteger(Boolean) _output_get) 0.005) 0.001 0.01) :!class /Script/Engine.KismetMaterialLibrary))
  (:Released
    (bind _output_get_2 (Variables|Default|SetForward false))
    (Rendering|Material|SetScalarParameterValue "/Game/Materials/mc_Opacity.mc_Opacity" "Opacity Scalar" (+ (* (Math|Conversions|ToInteger(Boolean) _output_get_2) 0.004) 0.0008) :!class /Script/Engine.KismetMaterialLibrary)))

(event Input|ActionEvents|InputActionBackwards
  (params (Key :type Key%20Structure :default "None"))
  (:Pressed
    (Variables|Default|SetBackward true))
  (:Released
    (Variables|Default|SetBackward false)))

(event Input|ActionEvents|InputActionPower-up
  (params (Key :type Key%20Structure :default "None"))
  (:Pressed
    (Development|PrintString "Using Power-Up")))

(event Input|AxisEvents|InputAxisPitch
  (params (AxisValue :type Float%20%28single-precision%29))
  ;[0 0.005721 1] Gets the Input for Pitch
  (bind _output_get (Variables|Default|SetPitch AxisValue))
  (Development|PrintString (Utilities|String|ToString(Float) _output_get)))

(event Input|AxisEvents|InputAxisRoll2
  (params (AxisValue :type Float%20%28single-precision%29))
  ;[0.09299 1 0] Gets the Input for the Rolls
  (if (>= (.z (Transformation|GetWorldLocation (Variables|Default|GetPlane))) 3e+01)
    (Variables|Default|SetRoll AxisValue)))

(event Input|AxisEvents|InputAxisYaw
  (params (AxisValue :type Float%20%28single-precision%29))
  ;[1 0.004069 0] Gets the Input for the YAW
  (Variables|Default|SetYaw AxisValue))

(fn ConstructionScript)

(fn ThrottleInput
  (if (Variables|Default|GetForward)
    ;[1 1 1] Have the player decrease speed with backwards, but not allow them to reverse in the race
    (bind _result (Math|Integer|IncrementInt (Variables|Default|GetSpeed))
      (:%20%20
        (Variables|Default|SetSpeed (Math|Integer|Clamp(Integer) _result 0 100))))
    (else
      (if (Variables|Default|GetBackward)
        _
        (else
          _))
      (bind _result_2 (Math|Integer|DecrementInt (Variables|Default|GetSpeed))
        (:%20%20
          (Variables|Default|SetSpeed (Math|Integer|Clamp(Integer) _result_2 0 100)))))))

(fn CalculateSpeed
  (bind _plane (Variables|Default|GetPlane))
  (bind _returnvalue (Physics|GetPhysicsLinearVelocity _plane "None"))
  (Physics|SetPhysicsLinearVelocity (Variables|Default|GetPlane) (Math|Vector|Lerp(Vector) _returnvalue (* (Math|Vector|GetForwardVector _plane) (Math|Float|Clamp(Float) (* (Variables|Default|GetSpeed) 5.0) 0.0 3.5e+02)) 0.5) false "None"))

(fn ApplyTurning
  (bind _plane (Variables|Default|GetPlane))
  (bind _returnvalue (Transformation|GetWorldRotation _plane))
  ;[1 0 0.6829] Add to Angular Velocity
  (Class|PrimitiveComponent|SetPhysicsAngularVelocityinDegrees (Variables|Default|GetPlane) (+ (* (Math|Vector|GetRightVector _returnvalue) (* (Variables|Default|GetPitch) (Variables|Default|GetAirControl))) (* (Math|Vector|GetForwardVector _returnvalue) (* (Variables|Default|GetRoll) (Variables|Default|GetAirControl))) (* (Math|Vector|GetUpVector _returnvalue) (* (Variables|Default|GetYaw) (Variables|Default|GetAirControl)))) false "None"))