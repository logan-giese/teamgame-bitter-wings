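; Homing missile actor that tracks an enemy plane using its projectile movement component.
; The HomingMissile event stores the enemy's PlaneRef as Target and assigns it as the homing component.
; Each Tick rebuilds the missile's rotation from its axis vectors scaled by its rotation delta to Target.
; Overlaps with non-friendly actors only print the location, as the impulse, explosion and destroy logic is disconnected.
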(event OnComponentHit(Capsule)
  (params (HitComponent :type Primitive%20Component%20Object%20Reference) (OtherActor :type Actor%20Object%20Reference) (OtherComp :type Primitive%20Component%20Object%20Reference) (NormalImpulse :type Vector :default "0, 0, 0") (Hit :type Hit%20Result%20Structure%20%28by%20ref%29)))

(event Custom|HomingMissile
  (params (EnemyActor :type Flying%20BP%20Object%20Reference) (Enemy :type Static%20Mesh%20Actor%20Object%20Reference))
  ;[0 0.2872 1] Sets the Homing Missile
  (if (Utilities|IsValid EnemyActor)
    (bind _output_get (Variables|Default|SetTarget (Variables|/Game/Blueprints/Flying_BP.Flying_BP_C|GetPlane_Ref EnemyActor)))
    (Variables|/Script/Engine.ProjectileMovementComponent|SetHomingTargetComponent (Variables|Default|GetProjectile) _output_get)))

(event EventBeginPlay)

(event Collision|EventActorBeginOverlap
  (params (OtherActor :type Actor%20Object%20Reference))
  ;[0 0.935 1] Adds impulse on hit and spawns emmiter before destroying
  (if (!= OtherActor (Variables|Default|GetFriendly))
    (Development|PrintString (Utilities|String|Append (Utilities|String|ToString(Vector) (Transformation|GetActorLocation)) "Hit Location for Missile"))))

(event EventTick
  (params (DeltaSeconds :type Float%20%28single-precision%29))
  (CallFunction|UpdateWorldRotation))

(fn ConstructionScript)

(fn UpdateWorldRotation
  (bind _target (Variables|Default|GetTarget))
  (bind _missile (Variables|Default|GetMissile))
  (bind _missile_2 (Variables|Default|GetMissile))
  (bind _returnvalue (Transformation|GetWorldRotation _missile))
  (bind _returnvalue_2 (Transformation|GetWorldRotation _missile_2))
  (bind _returnvalue_3 (Transformation|GetWorldRotation _target))
  (bind _returnvalue_4 (Math|Rotator|Delta(Rotator) _returnvalue_3 _returnvalue))
  (Transformation|SetWorldRotation (Variables|Default|GetMissile) (Math|Rotator|MakeRotationfromAxes (* (Math|Vector|GetForwardVector _returnvalue_2) (.roll _returnvalue_4)) (* (Math|Vector|GetRightVector _returnvalue_2) (.pitch _returnvalue_4)) (* (Math|Vector|GetUpVector _returnvalue_2) (.yaw _returnvalue_4))) false false))