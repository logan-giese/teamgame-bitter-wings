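; Trigger volume that sets a racer's HitCount to a fixed value, apparently as stuck or collision handling.
; The construction script snaps the Box to the referenced mesh actor's transform with padded scale, and BeginPlay enlarges it again.
; On overlap it prints a debug message, then waits briefly before writing HitCount on any Flying_BP actor tagged "racer".
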(event EventBeginPlay
  (bind _box (Variables|Default|GetBox))
  (bind _returnvalue (Transformation|GetWorldTransform _box))
  (bind (_location _rotation _scale) (Math|Transform|BreakTransform _returnvalue))
  (Transformation|SetWorldTransform _box (Math|Transform|MakeTransform _location _rotation (+ _scale "2.000000,2.000000,2.000000")) false false))

(event EventTick
  (params (DeltaSeconds :type Float%20%28single-precision%29)))

(event Collision|EventActorBeginOverlap
  (params (OtherActor :type Actor%20Object%20Reference))
  (Development|PrintString "Hit")
  (if (Actor|ActorHasTag OtherActor "racer")
    (bind _asflying_bp (Utilities|Casting|CastToFlying_BP OtherActor))
    (Utilities|FlowControl|Delay 1.0)
    (Variables|/Game/Blueprints/Flying_BP.Flying_BP_C|SetHitCount _asflying_bp 3)))

(fn ConstructionScript
  (bind _transform (Variables|Default|GetTransform))
  (bind _staticmeshcomponent (Variables|/Script/Engine.StaticMeshActor|GetStaticMeshComponent _transform))
  (bind _returnvalue (Transformation|GetWorldTransform _staticmeshcomponent))
  (bind (_location _rotation _scale) (Math|Transform|BreakTransform _returnvalue))
  (if (Utilities|IsValid _transform)
    (Transformation|SetWorldTransform (Variables|Default|GetBox) (Math|Transform|MakeTransform _location _rotation (+ _scale "2.000000,2.000000,2.000000")) false false)))