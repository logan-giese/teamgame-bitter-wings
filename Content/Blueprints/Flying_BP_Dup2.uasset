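; Flyable plane racer, driven by player input or AI steering toward a target, with power-up pickups.
; Each tick sets physics angular velocity from pitch, roll and yaw, scaled by altitude, and blends linear velocity toward the forward vector.
; A looping timer ramps player throttle, while throttle input drives smoke opacity through a material parameter collection.
; Power-ups offer a timed speed boost or homing missile at the nearest plane, though pickups currently always grant missiles.
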(event Custom|Wireless
  ;[0.6094 0.5243 0.02508] Will claculate the steering for the AI and then set the speed, Yaw, and Pitch for the AI
  (Utilities|FlowControl|Sequence
    (:then_0
      (bind (_pitch _yaw) (Utilities|SteeringCalc)))
    (:then_1
      (Variables|Default|SetSpeed 1000) ; Had to set to a really hig value to then use clamp in set speed. Arbitrary value here
      (Variables|Default|SetYaw _yaw)
      (Variables|Default|SetPitch _pitch))))

(event Custom|Waiting
  (params (Timer :type Float%20%28single-precision%29))
  (Utilities|FlowControl|Delay Timer))

(event Collision|EventActorBeginOverlap
  (params (OtherActor :type Actor%20Object%20Reference))
  ;[0.2083 0.3089 1 1 20] For when the racer overlaps with either a powerup or another racer
  (|CheckPowerUpTag OtherActor
    (:True%20Execute
      (CallFunction|GeneratePowerUp)
      (CallFunction|HidePowerup OtherActor true)
      (Utilities|FlowControl|Delay 5.0)
      (CallFunction|HidePowerup OtherActor false))
    (:False%20Execute
      (|RacerCheckup OtherActor
        (:True%20Execute
          (Development|PrintString "Hit Other Racer"))
        (:False%20Execute
          (Development|PrintString "Hit PowerUp"))))))

(event EventBeginPlay
  (Variables|Default|SetOpacityVar "/Game/Materials/m_SMoke.m_Smoke")
  (|PlayerCheck))

(event EventTick
  (params (DeltaSeconds :type Float%20%28single-precision%29))
  (if (Variables|Default|GetisAI)
    (CallFunction|Wireless))
  ;[0.7317 1 0.2878] Changes the air control variable for takeoff and for flying to make it slower in air
  (if (< (.z (Transformation|GetWorldLocation (Variables|Default|GetPlane))) 3e+01)
    (Variables|Default|SetAirControl 1.65e+03)
    (else
      (Variables|Default|SetAirControl 7e+01)))
  (CallFunction|ApplyTurning)
  (CallFunction|CalculateSpeed))

(event Input|ActionEvents|InputActionForward
  (params (Key :type Key%20Structure :default "None"))
  (:Pressed
    (bind _output_get (Variables|Default|SetForward true))
    ;[1 1 1] Smoke trails defined by throttle bool only
    (Rendering|Material|SetScalarParameterValue "/Game/Materials/mc_Opacity.mc_Opacity" "Opacity Scalar" (Math|Float|Clamp(Float) (* (Math|Conversions|ToInteger(Boolean) _output_get) 0.005) 0.01 0.02) :!class /Script/Engine.KismetMaterialLibrary))
  (:Released
    (bind _output_get_2 (Variables|Default|SetForward false))
    (Rendering|Material|SetScalarParameterValue "/Game/Materials/mc_Opacity.mc_Opacity" "Opacity Scalar" (+ (* (Math|Conversions|ToInteger(Boolean) _output_get_2) 0.004) 0.0008) :!class /Script/Engine.KismetMaterialLibrary)))

(event Input|ActionEvents|InputActionBackwards
  (params (Key :type Key%20Structure :default "None"))
  (:Pressed
    (Variables|Default|SetBackward true))
  (:Released
    (Variables|Default|SetBackward false)))

(event Input|ActionEvents|InputActionPower-up
  (params (Key :type Key%20Structure :default "None"))
  (:Pressed
    (bind _speedflag (CallFunction|UsePowerup))
    (if _speedflag
      (Utilities|FlowControl|Delay 5.0)
      (Variables|Default|SetSpeedMulti 2e+02)
      (Development|PrintString "Speed Boost Ended"))))

(event Input|AxisEvents|InputAxisPitch
  (params (AxisValue :type Float%20%28single-precision%29))
  ;[0 0.005721 1] Gets the Input for Pitch
  (Variables|Default|SetPitch AxisValue))

(event Input|AxisEvents|InputAxisRoll2
  (params (AxisValue :type Float%20%28single-precision%29))
  ;[0.09299 1 0] Gets the Input for the Rolls
  (if true
    (Variables|Default|SetRoll AxisValue)))

(event Input|AxisEvents|InputAxisYaw
  (params (AxisValue :type Float%20%28single-precision%29))
  ;[1 0.004069 0] Gets the Input for the YAW
  (Variables|Default|SetYaw AxisValue))

(fn ConstructionScript)

(fn ThrottleInput
  (if (Variables|Default|GetForward)
    ;[1 1 1] Have the player decrease speed with backwards, but not allow them to reverse in the race
    (bind _result (Math|Integer|IncrementInt (Variables|Default|GetSpeed))
      (:%20%20
        (Variables|Default|SetSpeed (Math|Integer|Clamp(Integer) _result 0 200))))
    (else
      (if (Variables|Default|GetBackward)
        _
        (else
          _))
      (bind _result_2 (Math|Integer|DecrementInt (Variables|Default|GetSpeed))
        (:%20%20
          (Variables|Default|SetSpeed (Math|Integer|Clamp(Integer) _result_2 0 100)))))))

(fn CalculateSpeed
  (bind _plane (Variables|Default|GetPlane))
  (bind _plane_2 (Variables|Default|GetPlane))
  (if (Variables|Default|GetisAI)
    ;[1 1 1] Speed if AI
    (bind _returnvalue (Physics|GetPhysicsLinearVelocity _plane "None"))
    (Physics|SetPhysicsLinearVelocity (Variables|Default|GetPlane) (Math|Vector|Lerp(Vector) _returnvalue (* (Math|Vector|GetForwardVector _plane) (Math|Float|Clamp(Float) (Math|Random|RandomFloatinRange (* (Variables|Default|GetSpeed) 1.0) (* (Variables|Default|GetSpeed) 7.0)) 0.0 1.5e+02)) 0.5) false "None")
    (else
      ;[1 1 1] Speed if Player Controlled
      (bind _output_get (Variables|Default|SetSpeed (Math|Float|Truncate (* (Variables|Default|GetSpeed) 5.0))))
      (bind _returnvalue_2 (Physics|GetPhysicsLinearVelocity _plane_2 "None"))
      (Physics|SetPhysicsLinearVelocity (Variables|Default|GetPlane) (Math|Vector|Lerp(Vector) _returnvalue_2 (* (Math|Vector|GetForwardVector _plane_2) (Math|Float|Clamp(Float) (Math|Conversions|ToFloat(Integer) _output_get) 0.0 (Variables|Default|GetSpeedMulti))) 0.5) false "None"))))

(fn ApplyTurning
  (bind _plane (Variables|Default|GetPlane))
  (bind _returnvalue (Transformation|GetWorldRotation _plane))
  ;[1 0 0.6829] Add to Angular Velocity
  (Class|PrimitiveComponent|SetPhysicsAngularVelocityinDegrees (Variables|Default|GetPlane) (+ (* (Math|Vector|GetRightVector _returnvalue) (* (Variables|Default|GetPitch) (Variables|Default|GetAirControl))) (* (Math|Vector|GetForwardVector _returnvalue) (* (Variables|Default|GetRoll) (Variables|Default|GetAirControl))) (* (Math|Vector|GetUpVector _returnvalue) (* (Variables|Default|GetYaw) (Variables|Default|GetAirControl)))) false "None"))

(fn UsePowerup
  ;[0.9387 0.4735 0.4125] Determine type of powerup
  (switch int (Variables|Default|GetPowerupType)
    (:Default
      (Development|PrintString "Error: PowerupType is not being instanciated through the editor"))
    (:0
      (Development|PrintString "No Power-Up to use"))
    (:1
      ;[1 1 1] Speed Power-Up
      (Development|PrintString "Speed Boost")
      (Variables|Default|SetSpeedMulti 275.0)
      (bind _output_get (LocalVariables|SetisSpeedBoost true))
      (Variables|Default|SetPowerupType 3 :!label _label)
      (return _output_get))
    (:3
      ;[1 1 1] Missile Power-Up
      (CallFunction|FindNearest)
      (bind _transform (CallFunction|SetMissileTransform))
      (bind _returnvalue (Game|SpawnActorfromClass "/Game/Blueprints/Missile_BP.Missile_BP_C" _transform "Undefined" 0 0))
      (Default|HomingMissile _returnvalue (Variables|Default|GetEnemy) self)
      (goto _label))))

(fn HidePowerup
  (params (Powerup :type Actor%20Object%20Reference) (Set :type Boolean))
  (Rendering|SetActorHiddenInGame Powerup Set))

(fn GeneratePowerUp
  (Variables|Default|SetPowerupType 3))

(fn FindNearest
  (bind _outactors (Actor|GetAllActorsOfClass "/Game/Blueprints/Flying_BP.Flying_BP_C"))
  (for _array_element _outactors
    (if (and (< (Math|Vector|VectorLength (- (Transformation|GetActorLocation _array_element) (Transformation|GetActorLocation self))) (LocalVariables|GetCurrentSmallest)) (!= _array_element self))
      (LocalVariables|SetCurrentSmallest (Math|Vector|VectorLength (- (Transformation|GetActorLocation _array_element) (Transformation|GetActorLocation self))))
      (Variables|Default|SetEnemy _array_element)))
  (Variables|Default|SetDistance (LocalVariables|GetCurrentSmallest)))

(fn SetMissileTransform
  (bind _plane_ref (Variables|Default|GetPlane_Ref))
  (bind _returnvalue (Transformation|GetWorldTransform _plane_ref))
  (return (Math|Transform|MakeTransform (+ (.location _returnvalue) (- (Math|Vector|GetUpVector (.rotation _returnvalue)) 2e+01)) (.rotation _returnvalue) (.scale _returnvalue))))