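; MusicManager plays the game's background music and switches it between four stations.
; BeginPlay sets the base volume sound mix, then creates and plays a 2D sound from the first track of Station 1, keeping it as BackgroundMusic.
; ChangeStation stops and destroys that component, then maps a 1-based station number to a new 2D sound, always using that station's first track.
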(event EventBeginPlay
  (Class|GameplayStatics|SetBaseSoundMix "/Game/Audio/VolumeMix.VolumeMix") ; Activate volume sound mix
  (bind _returnvalue (Audio|CreateSound2D (Utilities|Array|Get(acopy) (Variables|RadioStations|Getstation1)) 1.0 1.0 0.0 0))
  (bind _output_get (Variables|Default|SetbackgroundMusic _returnvalue))
  (Audio|Components|Audio|Play _output_get 0.0) ; Play the starting background music
)

(event EventTick
  (params (DeltaSeconds :type Float%20%28single-precision%29)))

(fn ConstructionScript)

(fn ChangeStation
  (params (stationNumber :type Integer))
  (Audio|Components|Audio|Stop (Variables|Default|GetbackgroundMusic)) ; Stop the current background music
  (Components|DestroyComponent (Variables|Default|GetbackgroundMusic))
  (switch int (- stationNumber 1)
    (:0
      (bind _returnvalue (Audio|CreateSound2D (Utilities|Array|Get(acopy) (Variables|RadioStations|Getstation1)) 1.0 1.0 0.0 0))
      (Variables|Default|SetbackgroundMusic _returnvalue))
    (:1
      (bind _returnvalue_2 (Audio|CreateSound2D (Utilities|Array|Get(acopy) (Variables|RadioStations|Getstation2)) 1.0 1.0 0.0 0))
      (Variables|Default|SetbackgroundMusic _returnvalue_2))
    (:2
      (bind _returnvalue_3 (Audio|CreateSound2D (Utilities|Array|Get(acopy) (Variables|RadioStations|Getstation3)) 1.0 1.0 0.0 0))
      (Variables|Default|SetbackgroundMusic _returnvalue_3))
    (:3
      (bind _returnvalue_4 (Audio|CreateSound2D (Utilities|Array|Get(acopy) (Variables|RadioStations|Getstation4)) 1.0 1.0 0.0 0))
      (Variables|Default|SetbackgroundMusic _returnvalue_4)))
  (Audio|Components|Audio|Play (Variables|Default|GetbackgroundMusic) 0.0) ; Play the new background music
)