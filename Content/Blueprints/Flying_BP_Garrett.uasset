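; Physics-driven plane racer for a flying race, controlled by either player input or AI steering toward a target.
; Tick applies pitch, roll and yaw as angular velocity, with altitude-based control strength, and blends linear velocity toward clamped forward speed.
; A looping timer drives player throttle, while throttle input also sets smoke-trail opacity.
; Overlapped pickups grant power-ups; handlers cover boost, homing projectiles and area slowdown, though generation currently yields only the slowdown.
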(event Custom|Wireless
  ;[0.6094 0.5243 0.02508] Will claculate the steering for the AI and then set the speed, Yaw, and Pitch for the AI
  (Utilities|FlowControl|Sequence
    (:then_0
      (bind (_pitch _yaw) (Utilities|SteeringCalc)))
    (:then_1
      (Variables|Movement|SetSpeed 1000) ; Had to set to a really hig value to then use clamp in set speed. Arbitrary value here
      (Variables|Movement|SetYaw _yaw)
      (Variables|Movement|SetPitch _pitch))))

(event Custom|Restart
  ;[1 1 1] Race Events - TODO
)

(event Custom|UpdateLap
  ;[1 1 1] Race Events - TODO
)

(event Custom|Respawn
  ;[1 1 1] Race Events - TODO
)

(event Collision|EventActorBeginOverlap
  (params (OtherActor :type Actor%20Object%20Reference))
  ;[0.2083 0.3089 1 1 20] For when the racer overlaps with either a powerup or another racer
  (|CheckPowerUpTag OtherActor
    (:True%20Execute
      (CallFunction|GeneratePowerUp)
      (CallFunction|HidePowerup OtherActor true)
      (Utilities|FlowControl|Delay 5.0)
      (CallFunction|HidePowerup OtherActor false))
    (:False%20Execute
      (|RacerCheckup OtherActor
        (:True%20Execute
          (Development|PrintString "Hit Other Racer"))))))

(event EventBeginPlay
  (Variables|Default|SetOpacityVar "/Game/Materials/m_SMoke.m_Smoke")
  (|PlayerCheck))

(event EventTick
  (params (DeltaSeconds :type Float%20%28single-precision%29))
  (if (Variables|Default|GetisAI)
    (CallFunction|Wireless))
  ;[0.7317 1 0.2878] Changes the air control variable for takeoff and for flying to make it slower in air
  (if (< (.z (Transformation|GetWorldLocation (Variables|Default|GetPlane))) 3e+01)
    (Variables|Movement|SetAirControl 1.65e+03)
    (else
      (Variables|Movement|SetAirControl 7e+01)))
  (CallFunction|ApplyTurning)
  (CallFunction|CalculateSpeed))

(event Input|ActionEvents|InputActionForward
  (params (Key :type Key%20Structure))
  (:Pressed
    (bind _output_get (Variables|Movement|SetForward true))
    ;[1 1 1] Smoke trails defined by throttle bool only
    (Rendering|Material|SetScalarParameterValue "/Game/Materials/mc_Opacity.mc_Opacity" "Opacity Scalar" (Math|Float|Clamp(Float) (* (Math|Conversions|ToInteger(Boolean) _output_get) 0.005) 0.01 0.02) :!class /Script/Engine.KismetMaterialLibrary))
  (:Released
    (bind _output_get_2 (Variables|Movement|SetForward false))
    (Rendering|Material|SetScalarParameterValue "/Game/Materials/mc_Opacity.mc_Opacity" "Opacity Scalar" (+ (* (Math|Conversions|ToInteger(Boolean) _output_get_2) 0.004) 0.0008) :!class /Script/Engine.KismetMaterialLibrary)))

(event Input|ActionEvents|InputActionBackwards
  (params (Key :type Key%20Structure))
  (:Pressed
    (Variables|Movement|SetBackward true))
  (:Released
    (Variables|Movement|SetBackward false)))

(event Input|ActionEvents|InputActionPower-up
  (params (Key :type Key%20Structure))
  (:Pressed
    (bind _speedflag (CallFunction|UsePowerup))
    (if _speedflag
      (Utilities|FlowControl|Delay 5.0)
      (Variables|Default|SetSpeedMulti 2e+02)
      (Development|PrintString "Speed Boost Ended"))))

(event Input|AxisEvents|InputAxisPitch
  (params (AxisValue :type Float%20%28single-precision%29))
  ;[0 0.005721 1] Gets the Input for Pitch
  (Variables|Movement|SetPitch AxisValue))

(event Input|AxisEvents|InputAxisRoll2
  (params (AxisValue :type Float%20%28single-precision%29))
  ;[0.09299 1 0] Gets the Input for the Rolls
  (if true
    (Variables|Movement|SetRoll AxisValue)))

(event Input|AxisEvents|InputAxisYaw
  (params (AxisValue :type Float%20%28single-precision%29))
  ;[1 0.004069 0] Gets the Input for the YAW
  (Variables|Movement|SetYaw AxisValue))

(fn ConstructionScript)

(fn ThrottleInput
  (if (Variables|Movement|GetForward)
    ;[1 1 1] Have the player decrease speed with backwards, but not allow them to reverse in the race
    (bind _result (Math|Integer|IncrementInt (Variables|Movement|GetSpeed))
      (:%20%20
        (Variables|Movement|SetSpeed (Math|Integer|Clamp(Integer) _result 0 200))))
    (else
      (if (Variables|Movement|GetBackward)
        _
        (else
          _))
      (bind _result_2 (Math|Integer|DecrementInt (Variables|Movement|GetSpeed))
        (:%20%20
          (Variables|Movement|SetSpeed (Math|Integer|Clamp(Integer) _result_2 0 100)))))))

(fn CalculateSpeed
  (bind _plane (Variables|Default|GetPlane))
  (bind _speed (Variables|Movement|GetSpeed))
  (bind _plane_2 (Variables|Default|GetPlane))
  (if (Variables|Default|GetisAI)
    ;[0.5219 0.03349 0] Speed if AI
    (bind _returnvalue (Physics|GetPhysicsLinearVelocity _plane "None"))
    (Physics|SetPhysicsLinearVelocity (Variables|Default|GetPlane) (Math|Vector|Lerp(Vector) _returnvalue (* (Math|Vector|GetForwardVector _plane) (Math|Float|Clamp(Float) (Math|Random|RandomFloatinRange (* _speed 1.0) (* _speed 7.0)) 0.0 (Variables|Default|GetSpeedMulti))) 0.5) false "None")
    (else
      ;[0 0.2969 0.03432] Speed if Player Controlled
      (bind _returnvalue_2 (Physics|GetPhysicsLinearVelocity _plane_2 "None"))
      (Physics|SetPhysicsLinearVelocity (Variables|Default|GetPlane) (Math|Vector|Lerp(Vector) _returnvalue_2 (* (Math|Vector|GetForwardVector _plane_2) (Math|Float|Clamp(Float) (Math|Conversions|ToFloat(Integer) (Math|Float|Truncate (* (Variables|Movement|GetSpeed) 5.0))) 0.0 (Variables|Default|GetSpeedMulti))) 0.5) false "None"))))

(fn ApplyTurning
  (bind _plane (Variables|Default|GetPlane))
  (bind _returnvalue (Transformation|GetWorldRotation _plane))
  ;[1 0 0.6829] Add to Angular Velocity
  (Class|PrimitiveComponent|SetPhysicsAngularVelocityinDegrees (Variables|Default|GetPlane) (+ (* (Math|Vector|GetRightVector _returnvalue) (* (Variables|Movement|GetPitch) (Variables|Movement|GetAirControl))) (* (Math|Vector|GetForwardVector _returnvalue) (* (Variables|Movement|GetRoll) (Variables|Movement|GetAirControl))) (* (Math|Vector|GetUpVector _returnvalue) (* (Variables|Movement|GetYaw) (Variables|Movement|GetAirControl)))) false "None"))

(fn UsePowerup
  ;[0.9387 0.4735 0.4125] Determine type of powerup
  (switch int (Variables|Default|GetPowerupType)
    (:Default
      (Development|PrintString "Error: PowerupType is not being instanciated through the editor"))
    (:0
      (Development|PrintString "No Power-Up to use"))
    (:1
      ;[1 0.5831 0.1336] Speed Power-Up
      (Development|PrintString "Speed Boost")
      (Variables|Default|SetSpeedMulti 275.0)
      (bind _output_get (LocalVariables|SetisSpeedBoost true))
      (Variables|Default|SetPowerupType 4 :!label _label)
      (return _output_get))
    (:2
      ;[0.1899 1 0.7001] Gummy Bears Power-Up
      (CallFunction|FindNearest)
      (if (Utilities|IsValid (Variables|Default|GetEnemy))
        (bind _transform (CallFunction|SetMissileTransform))
        (bind _returnvalue (Game|SpawnActorfromClass "/Game/Blueprints/GummyBear_BP.GummyBear_BP_C" _transform "Undefined" 0 0))
        (Default|HomingMissile _returnvalue (Variables|Default|GetEnemy) self)
        (Audio|PlaySoundatLocation "/Game/StarterContent/Audio/Steam01.Steam01" (Transformation|GetActorLocation) "0, 0, 0" 0.1 1.0 0.0 0 0 0)
        (goto _label)
        (else
          (Development|PrintString "Enemy not found"))))
    (:3
      ;[0.8402 0.03048 1] Missile Power-Up
      (CallFunction|FindNearest)
      (if (Utilities|IsValid (Variables|Default|GetEnemy))
        (bind _transform_2 (CallFunction|SetMissileTransform))
        (bind _returnvalue_2 (Game|SpawnActorfromClass "/Game/Blueprints/Missile_BP.Missile_BP_C" _transform_2 "Undefined" 0 0))
        (Default|HomingMissile _returnvalue_2 (Variables|Default|GetEnemy) self)
        (Audio|PlaySoundatLocation "/Game/StarterContent/Audio/Explosion01.Explosion01" (Transformation|GetActorLocation) "0, 0, 0" 0.1 1.0 0.0 0 0 0)
        (goto _label)
        (else
          (Development|PrintString "Enemy not found"))))
    (:4
      ;[0.02521 0.4201 1] Skeaker Drop Power-up
      (bind _closeenemies (CallFunction|FindAllinRange 2.5e+02))
      (CallFunction|EMPEnemies _closeenemies)
      (Effects|SpawnEmitterAttached "/Game/StarterContent/Particles/P_Sparks.P_Sparks" 0 "None" (Transformation|GetWorldLocation (Variables|Default|GetPlane_Ref)))
      (Audio|SpawnSoundAttached "/Game/StarterContent/Audio/Collapse_Cue.Collapse_Cue" 0 "None" "0, 0, 0" "0, 0, 0" "KeepRelativeOffset" false 1.0 1.0 0.0 0 0)
      (Development|PrintString "Kicker Audio Vibes")
      (goto _label))))

(fn HidePowerup
  (params (Powerup :type Actor%20Object%20Reference) (Set :type Boolean))
  (Rendering|SetActorHiddenInGame Powerup Set))

(fn GeneratePowerUp
  (if (> (Math|Integer|%(Integer) (Math|Random|RandomInteger 100) 5) 1)
    (Variables|Default|SetPowerupType 4)
    (else
      (CallFunction|GeneratePowerUp))))

(fn FindNearest
  (bind _self self)
  (bind _returnvalue (Transformation|GetActorLocation _self))
  (bind _outactors (Actor|GetAllActorsOfClasswithTag "/Game/Blueprints/Flying_BP.Flying_BP_C" "racer"))
  (for _array_element _outactors
    (if (and (< (Math|Vector|VectorLength (- (Transformation|GetActorLocation _array_element) _returnvalue)) (LocalVariables|GetCurrentSmallest)) (Class|KismetMathLibrary|NotEqualExactlyVectorVector (Transformation|GetActorLocation _array_element) _returnvalue))
      (LocalVariables|SetCurrentSmallest (Math|Vector|VectorLength (- (Transformation|GetActorLocation _array_element) _returnvalue)))
      (Variables|Default|SetEnemy _array_element))))

(fn SetMissileTransform
  (bind _plane (Variables|Default|GetPlane))
  (bind _returnvalue (Transformation|GetWorldTransform _plane))
  (return (Math|Transform|MakeTransform (- (.location _returnvalue) (* (Math|Vector|GetUpVector (.rotation _returnvalue)) 7.5)) (.rotation _returnvalue) "0.100000,0.100000,0.100000")))

(fn FindAllinRange
  (params (Area :type Float%20%28single-precision%29))
  (bind _self self)
  (bind _returnvalue (Transformation|GetActorLocation _self))
  (bind _outactors (Actor|GetAllActorsOfClasswithTag "/Game/Blueprints/Flying_BP.Flying_BP_C" "racer"))
  (for _array_element _outactors
    (if (and (<= (Math|Vector|VectorLength (- (Transformation|GetActorLocation _array_element) _returnvalue)) Area) (Class|KismetMathLibrary|NotEqualExactlyVectorVector (Transformation|GetActorLocation _array_element) _returnvalue))
      (Utilities|Array|Add (LocalVariables|GetEnemyArray) _array_element)))
  (return (LocalVariables|GetEnemyArray)))

(fn EMPEnemies
  (params (Enemies :type Array%20of%20Flying%20BP%20Object%20References))
  (for _array_element Enemies
    (Variables|/Game/Blueprints/Flying_BP.Flying_BP_C|SetSpeedMulti _array_element 75.0)
    (Development|PrintString "Slowing enemy")))