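; Homing missile actor that flies at an enemy plane and explodes when it overlaps something.
; The HomingMissile event points the projectile component's homing target at the given enemy's PlaneRef, if that enemy is valid.
; Tick adds a fixed roll through SetActorRotation to spin the missile.
; Actor or capsule overlap triggers a one-time radial impulse and explosion emitter, then destroys the missile.
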(event OnComponentBeginOverlap(Capsule)
  (params (OverlappedComponent :type Primitive%20Component%20Object%20Reference) (OtherActor :type Actor%20Object%20Reference) (OtherComp :type Primitive%20Component%20Object%20Reference) (OtherBodyIndex :type Integer) (bFromSweep :type Boolean) (SweepResult :type Hit%20Result%20Structure%20%28by%20ref%29))
  (bind _radialforce (Variables|Default|GetRadialForce))
  ;[0 0.935 1] Adds impulse on hit and spawns emmiter before destroying
  (Development|PrintString "Hello")
  (Utilities|FlowControl|DoOnce false
    (:Completed
      (Class|RadialForceComponent|FireImpulse _radialforce)
      (Effects|SpawnEmitteratLocation "/Game/StarterContent/Particles/P_Explosion.P_Explosion" (Transformation|GetWorldLocation _radialforce))
      (Development|PrintString "Hit Enemy")
      (Actor|DestroyActor))))

(event Custom|HomingMissile
  (params (EnemyActor :type Flying%20BP%20Object%20Reference) (FriendlyActor :type Flying%20BP%20Object%20Reference))
  ;[0 0.2872 1] Sets the Homing Missile
  (if (Utilities|IsValid EnemyActor)
    (bind _output_get (Variables|Default|SetTarget (Variables|/Game/Blueprints/Flying_BP.Flying_BP_C|GetPlane_Ref EnemyActor)))
    (Variables|/Script/Engine.ProjectileMovementComponent|SetHomingTargetComponent (Variables|Default|GetProjectile) _output_get)
    (else
      (Development|PrintString "Invalid Enemy"))))

(event EventBeginPlay)

(event Collision|EventActorBeginOverlap
  (params (OtherActor :type Actor%20Object%20Reference))
  (bind _radialforce (Variables|Default|GetRadialForce))
  ;[0 0.935 1] Adds impulse on hit and spawns emmiter before destroying
  (Development|PrintString "Hello")
  (Utilities|FlowControl|DoOnce false
    (:Completed
      (Class|RadialForceComponent|FireImpulse _radialforce)
      (Effects|SpawnEmitteratLocation "/Game/StarterContent/Particles/P_Explosion.P_Explosion" (Transformation|GetWorldLocation _radialforce))
      (Development|PrintString "Hit Enemy")
      (Actor|DestroyActor))))

(event EventTick
  (params (DeltaSeconds :type Float%20%28single-precision%29))
  (CallFunction|UpdateRollRotation) ; Makes the missile very laggy in how it updates, and possible could not be updating the rotation
)

(fn ConstructionScript)

(fn UpdateRollRotation
  (bind _returnvalue (Transformation|GetActorRotation))
  (bind (_roll _pitch _yaw) (Math|Rotator|BreakRotator _returnvalue))
  (Transformation|SetActorRotation (Math|Rotator|MakeRotator (+ _roll 5.0) _pitch _yaw)))