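; Checkpoint tracker that runs a lap-based race for the Flying_BP player pawn.
; On BeginPlay it numbers the checkpoint array, activates the first ring and trigger, and binds each checkpoint's cleared event.
; Each clear plays a sound, then activates the next checkpoint and updates the pawn's respawn transform.
; At the last checkpoint it either flags the race complete on the pawn or loops to the first and increments the lap.
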(event Custom|ApplySettings)

(event Custom|StartSequence
  (bind _checkpoints (Variables|Checkpoints|GetCheckpoints))
  ;[1 1 1] Start sequence / Initializes checkpoints
  (for (_array_element _array_index) _checkpoints
    (Variables|/Game/Blueprints/CheckpointRing.CheckpointRing_C|SetCheckpointNumber _array_element (+ _array_index 1)) ; Set each checkpoint's number
  )
  (Variables|Default|SetTotalCheckpoints (Utilities|Array|Length _checkpoints))
  (CallFunction|ActivateCheckpoint (Utilities|Array|Get(acopy) _checkpoints)) ; Activate first checkpoint
  (for _array_element_2 (Variables|Checkpoints|GetCheckpoints)
    (EventDispatchers|BindEventtoCheckpointCleared _array_element_2 (delegate Custom|CheckpointClearedEvent))))

(event Custom|CheckpointClearedEvent
  (params (NextCheckpoint :type Integer))
  ;[1 1 1] Handle a checkpoint being cleared and test for race end
  (CallFunction|LapCheck NextCheckpoint)
  (Audio|Components|Audio|Play (Variables|/Script/Engine.AmbientSound|GetAudioComponent (Variables|RaceSettings|GetCheckpointSoundEffect)) 0.0) ; Play checkpoint sound effect
)

(event EventBeginPlay
  (bind _asflying_bp (Utilities|Casting|CastToFlying_BP (Game|Player|GetPlayerPawn 0)))
  (Variables|Default|SetPlayerPawnRef _asflying_bp) ; Store a reference to the player pawn
  (CallFunction|ApplySettings)
  (CallFunction|StartSequence))

(fn ConstructionScript)

(fn LapCheck
  (params (Checkpoint :type Integer))
  (bind _output_get (LocalVariables|SetLocalCheckpoint Checkpoint)) ; Checkpoint is next checkpoint
  (if (== _output_get (Variables|Default|GetTotalCheckpoints))
    (bind _isracecomplete (CallFunction|RaceCompleteCheck))
    (if _isracecomplete
      (Development|PrintString "RACE COMPLETE")
      (else
        (CallFunction|ActivateCheckpoint (Utilities|Array|Get(acopy) (Variables|Checkpoints|GetCheckpoints)))
        (Default|UpdateLap (Variables|Default|GetPlayerPawnRef))
        (Variables|/Game/Blueprints/Flying_BP.Flying_BP_C|SetRespawnLocation (Variables|Default|GetPlayerPawnRef) (Transformation|GetActorTransform (Utilities|Array|Get(acopy) (Variables|Checkpoints|GetCheckpoints) (- (LocalVariables|GetLocalCheckpoint) 1))) :!label _label)))
    (else
      (CallFunction|ActivateCheckpoint (Utilities|Array|Get(acopy) (Variables|Checkpoints|GetCheckpoints) (LocalVariables|GetLocalCheckpoint)))
      (goto _label))))

(fn ActivateCheckpoint
  (params (NextCheckpoint :type Checkpoint%20Ring%20Object%20Reference))
  (bind _trigger (Variables|/Game/Blueprints/CheckpointRing.CheckpointRing_C|GetTrigger NextCheckpoint))
  ;[1 1 1] Activate the next checkpoint (ring and overlap trigger)
  (Development|SetHiddeninGame _trigger false false)
  (Variables|/Script/Engine.PrimitiveComponent|SetbGenerateOverlapEvents _trigger true))

(fn RaceCompleteCheck
  (bind _playerpawnref (Variables|Default|GetPlayerPawnRef))
  (bind _playerpawnref_2 (Variables|Default|GetPlayerPawnRef))
  (if (>= (Variables|/Game/Blueprints/Flying_BP.Flying_BP_C|GetActualLap _playerpawnref_2) (Variables|/Game/Blueprints/Flying_BP.Flying_BP_C|GetMaxLaps _playerpawnref_2))
    (bind _output_get (Variables|/Game/Blueprints/Flying_BP.Flying_BP_C|SetRaceComplete _playerpawnref true))
    (LocalVariables|SetLocalComplete _output_get)
    (else
      (bind _output_get_2 (Variables|/Game/Blueprints/Flying_BP.Flying_BP_C|SetRaceComplete _playerpawnref false))
      (LocalVariables|SetLocalComplete _output_get_2)))
  (return (LocalVariables|GetLocalComplete)))