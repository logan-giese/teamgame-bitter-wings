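; Checkpoint ring for a flying race that the player's plane clears by passing through it in the correct direction.
; Every Flying_BP ending overlap with the trigger increments a place counter, whether AI or player.
; For the player, a velocity dot product against the Direction component gates clearing, which fires CheckpointCleared, hides the ring, deactivates it, writes the count to RacePlace and resets the counter.
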(event OnComponentEndOverlap(Trigger)
  (params (OverlappedComponent :type Primitive%20Component%20Object%20Reference) (OtherActor :type Actor%20Object%20Reference) (OtherComp :type Primitive%20Component%20Object%20Reference) (OtherBodyIndex :type Integer))
  ;[1 1 1] Clear checkpoint on end overlap
  (bind _asflying_bp (Utilities|Casting|CastToFlying_BP OtherActor)) ; Try casting actor to plane
  (Math|Integer|IncrementInt (Variables|Default|GetPlaceCounter) ; Add to place counter
    (:%20%20
      (if (Variables|Default|GetCheckpointActive)
        (bind _asflying_bp_2 (Utilities|Casting|CastToFlying_BP (Game|Player|GetPlayerPawn 0))) ; Check if it was the player
        (if (== _asflying_bp_2 _asflying_bp) ; Only disappear for the player, not AIs
          (if (> (Math|Vector|DotProduct (Transformation|GetVelocity _asflying_bp) (Math|Rotator|GetRotationXVector (Transformation|GetWorldRotation (Variables|Default|GetDirection)))) 0.0)
            (Default|CallCheckpointCleared (Variables|Default|GetCheckpointNumber)) ; Trigger checkpoint cleared event
            (Development|SetHiddeninGame (Variables|Default|GetTrigger) true false)
            (Variables|Default|SetCheckpointActive false)
            (CallFunction|SetRacePlacing)
            (Variables|Default|SetPlaceCounter 0)))))))

(fn ConstructionScript)

(fn SetRacePlacing
  (bind _asflying_bp (Utilities|Casting|CastToFlying_BP (Game|Player|GetPlayerPawn 0)))
  (Variables|/Game/Blueprints/Flying_BP.Flying_BP_C|SetRacePlace _asflying_bp (Variables|Default|GetPlaceCounter)))