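; Spline path actor that feeds a steering target to a referenced vehicle.
; Each tick it offsets the vehicle's location 500 units against the spline's local-space right vector at the nearest point, as a look-ahead.
; The spline point closest to that offset becomes the vehicle's Steering value and positions a sphere marker.
; An arrow sits at the spline point nearest the vehicle, oriented by that right vector with yaw turned 180 degrees.
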(event EventBeginPlay)

(event Collision|EventActorBeginOverlap
  (params (OtherActor :type Actor%20Object%20Reference)))

(event EventTick
  (params (DeltaSeconds :type Float%20%28single-precision%29))
  (bind _vehicleref (Variables|Default|GetVehicleRef))
  (bind _spline (Variables|Default|GetSpline))
  (bind _vehicleref_2 (Variables|Default|GetVehicleRef))
  (bind _returnvalue (Transformation|GetActorLocation _vehicleref))
  (bind _returnvalue_2 (Class|SplineComponent|FindRightVectorClosesttoWorldLocation _spline _returnvalue "Local"))
  (bind _returnvalue_3 (Math|Rotator|MakeRotationfromAxes _returnvalue_2 "0, 0, 0" "0, 0, 0"))
  (bind (_roll _pitch _yaw) (Math|Rotator|BreakRotator _returnvalue_3))
  (bind _output_get (Variables|/Game/Blueprints/Flying_BP.Flying_BP_C|SetSteering _vehicleref_2 (Spline|FindLocationClosesttoWorldLocation (Variables|Default|GetSpline) (- (Transformation|GetActorLocation (Variables|Default|GetVehicleRef)) (* (Math|Vector|GetForwardVector _returnvalue_3) 500)) "World")))
  (Transformation|SetWorldLocation (Variables|Default|GetSphere) _output_get false false)
  (Transformation|SetWorldLocationAndRotation (Variables|Default|GetArrow) (Spline|FindLocationClosesttoWorldLocation (Variables|Default|GetSpline) (Transformation|GetActorLocation _vehicleref_2) "World") (Math|Rotator|MakeRotator _roll _pitch (- _yaw 1.8e+02)) false false))

(fn ConstructionScript)