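; GummyBear_BP is a homing missile fired by one racer at another.
; HomingMissile stores the firer and sets the enemy's PlaneRef as the projectile's homing target.
; Tick caches the firer's position, so overlaps with "racer"-tagged actors count only when the missile is clear of it, then spawn steam and destroy the missile once.
; UpdateRollRotation adds a roll step but is not called here, and no hit impulse is applied despite the graph comment.
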(event Custom|HomingMissile
  (params (EnemyActor :type Flying%20BP%20Object%20Reference) (FriendlyActor :type Flying%20BP%20Object%20Reference))
  ;[0 0.2872 1] Sets the Homing Missile
  (if (Utilities|IsValid EnemyActor)
    (Variables|Default|SetFriendly FriendlyActor)
    (bind _output_get (Variables|Default|SetTarget (Variables|/Game/Blueprints/Flying_BP.Flying_BP_C|GetPlane_Ref EnemyActor)))
    (Variables|/Script/Engine.ProjectileMovementComponent|SetHomingTargetComponent (Variables|Default|GetProjectile) _output_get)
    (else
      (Development|PrintString "Invalid Enemy"))))

(event EventBeginPlay)

(event Collision|EventActorBeginOverlap
  (params (OtherActor :type Actor%20Object%20Reference))
  ;[0 0.935 1] Adds impulse on hit and spawns emmiter before destroying
  (if (and (Actor|ActorHasTag OtherActor "racer") (Math|Vector|NotEqual(Vector) (Variables|Default|GetFriendlyLocation) (Transformation|GetWorldLocation (Variables|Default|GetMissile)) 35.0))
    (Utilities|FlowControl|DoOnce false
      (:Completed
        (Effects|SpawnEmitteratLocation "/Game/StarterContent/Particles/P_Steam_Lit.P_Steam_Lit" (Transformation|GetWorldLocation (Variables|Default|GetDefaultSceneRoot)))
        (Actor|DestroyActor)))))

(event EventTick
  (params (DeltaSeconds :type Float%20%28single-precision%29))
  (Variables|Default|SetFriendlyLocation (Transformation|GetWorldLocation (Variables|/Game/Blueprints/Flying_BP.Flying_BP_C|GetPlane_Ref (Variables|Default|GetFriendly)))))

(fn ConstructionScript)

(fn UpdateRollRotation
  (bind _returnvalue (Transformation|GetActorRotation))
  (bind (_roll _pitch _yaw) (Math|Rotator|BreakRotator _returnvalue))
  (Transformation|SetActorRotation (Math|Rotator|MakeRotator (+ _roll 5.0) _pitch _yaw)))